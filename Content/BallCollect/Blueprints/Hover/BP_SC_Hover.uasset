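; BP_SC_Hover is a scene component that makes its owner's physics body hover above surfaces.
; It caches the owner's PrimitiveComponent at BeginPlay, then line-traces straight down in world space from its own location every Tick.
; On a hit, it pushes the body along the impact normal, with force fading linearly to zero at full trace length.
; A hit also applies linear and angular damping, which is never reset on a miss.
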(event EventBeginPlay
  (Variables|Default|SetPrimitiveComponent (Actor|GetComponentbyClass (Components|GetOwner) "/Script/Engine.PrimitiveComponent")))

(event EventTick
  (params (DeltaSeconds :type Float%20%28single-precision%29))
  (bind _returnvalue (Transformation|GetWorldLocation))
  (bind _primitivecomponent (Variables|Default|GetPrimitiveComponent))
  ;[1 1 1] Hover 悬浮
  (bind (_outhit _returnvalue_2) (Collision|LineTraceByChannel _returnvalue (- _returnvalue (Math|Vector|MakeVector 0.0 0.0 (Variables|Default|GetTraceLength))) "TraceTypeQuery1" false 0 "None"))
  (if _returnvalue_2
    (Physics|AddForce _primitivecomponent (* (.ImpactNormal (Collision|BreakHitResult _outhit)) (Math|Float|Lerp (Variables|Default|GetHoverForce) 0.0 (/ (Math|Vector|VectorLength (- (.Location (Collision|BreakHitResult _outhit)) (Transformation|GetWorldLocation))) (Variables|Default|GetTraceLength)))) "None" false)
    (Class|PrimitiveComponent|SetLinearDamping _primitivecomponent (Variables|Default|GetLinear%20Damping))
    (Class|PrimitiveComponent|SetAngularDamping (Variables|Default|GetPrimitiveComponent) (Variables|Default|GetAngular%20Damping))))