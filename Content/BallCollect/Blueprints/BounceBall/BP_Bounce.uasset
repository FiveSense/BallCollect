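; BP_Bounce is a bouncing ball actor for the BallCollect game that awards points when it hits another ball of its kind.
; On BeginPlay, a timeline drives the static mesh's world scale and a looping timer nudges the Sphere's rotation by small random amounts.
; Sphere hits on another BP_Bounce add to the score in BallGameMode and spawn a hit effect, while hits on Wall-tagged actors spawn a thunder-strike effect.
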(event OnComponentHit(Sphere)
  (params (HitComponent :type Primitive%20Component%20Object%20Reference) (OtherActor :type Actor%20Object%20Reference) (OtherComp :type Primitive%20Component%20Object%20Reference) (NormalImpulse :type Vector :default "0, 0, 0") (Hit :type Hit%20Result%20Structure%20%28by%20ref%29))
  (bind _returnvalue (Transformation|GetActorTransform))
  (bind _returnvalue_2 (Transformation|GetActorTransform))
  ;[1 1 1] 物体相互碰撞
  (Utilities|FlowControl|Sequence
    (:then_0
      (Utilities|Casting|CastToBP_Bounce OtherActor)
      ;;[0.007439 0 1] 物体碰撞到物体+2
      (bind _asball_game_mode (Utilities|Casting|CastToBallGameMode (Game|GetGameMode)))
      (Variables|/Game/BallCollect/Blueprints/GameFrame/BallGameMode.BallGameMode_C|SetScore _asball_game_mode (Utilities|Struct|MakeBP_Struct (+ (.score (Variables|/Game/BallCollect/Blueprints/GameFrame/BallGameMode.BallGameMode_C|GetScore _asball_game_mode)) 2) (.bulletnum (Variables|/Game/BallCollect/Blueprints/GameFrame/BallGameMode.BallGameMode_C|GetScore _asball_game_mode))))
      (Effects|SpawnEmitteratLocation "/Game/BallCollect/Blueprints/Particle/P_HitObject.P_HitObject" (.location _returnvalue_2) (.rotation _returnvalue_2)))
    (:then_1
      (if (Actor|ActorHasTag OtherActor "Wall")
        (Effects|SpawnEmitteratLocation "/Game/SimpleCartoonFX/FX/Thunder_Strike.Thunder_Strike" (.location _returnvalue) (.rotation _returnvalue))))))

(event Custom|Scale
  ;[1 1 1] Scale 0-1
  (bind _scale (Timeline|Timeline_0 PlayFromStart)
    (:Update
      (Transformation|SetWorldScale3D (Variables|Default|GetStaticMesh) (Math|Conversions|ToVector(Float) (/ _scale 2.0))))))

(event Custom|rotation
  (bind _returnvalue (Math|Random|RandomFloatinRange 0.0 1.0))
  ;[1 1 1] Random Rotate
  (Transformation|AddRelativeRotation (Variables|Default|GetSphere) (Math|Rotator|MakeRotator _returnvalue _returnvalue _returnvalue) false false))

(event EventBeginPlay
  (CallFunction|Scale)
  (Utilities|Time|SetTimerbyEvent (delegate Custom|rotation) 0.1 true))

(event Collision|EventActorBeginOverlap
  (params (OtherActor :type Actor%20Object%20Reference)))

(fn ConstructionScript)