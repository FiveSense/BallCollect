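; BP_Bullet is a bullet actor for BallCollect that spawns particle effects at its own position when its Sphere component hits something.
; Hitting a BP_Bounce spawns the Hit emitter, while hitting an actor tagged GlassWall spawns a steam effect, checked independently through a Sequence.
; The graph holds no movement, damage or destroy logic, and a disconnected copy of the GlassWall check never runs.
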(event OnComponentHit(Sphere)
  (params (HitComponent :type Primitive%20Component%20Object%20Reference) (OtherActor :type Actor%20Object%20Reference) (OtherComp :type Primitive%20Component%20Object%20Reference) (NormalImpulse :type Vector :default "0, 0, 0") (Hit :type Hit%20Result%20Structure%20%28by%20ref%29))
  (bind _returnvalue (Transformation|GetActorTransform))
  (bind _returnvalue_2 (Transformation|GetActorTransform))
  (Utilities|FlowControl|Sequence
    (:then_0
      (Utilities|Casting|CastToBP_Bounce OtherActor)
      (Effects|SpawnEmitteratLocation "/Game/SimpleCartoonFX/FX/Hit.Hit" (.location _returnvalue) (.rotation _returnvalue)))
    (:then_1
      (if (Actor|ActorHasTag OtherActor "GlassWall")
        (Effects|SpawnEmitteratLocation "/Game/BallCollect/Particles/P_Steam_Lit.P_Steam_Lit" (.location _returnvalue_2) (.rotation _returnvalue_2))))))

(event EventBeginPlay)

(event Collision|EventActorBeginOverlap
  (params (OtherActor :type Actor%20Object%20Reference)))

(event EventTick
  (params (DeltaSeconds :type Float%20%28single-precision%29)))

(fn ConstructionScript)