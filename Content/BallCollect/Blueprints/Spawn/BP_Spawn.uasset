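; BP_Spawn is a spawner actor that fills a box volume with BP_Bounce actors in the BallCollect game.
; When SpawnToggle is on at BeginPlay, a looping timer calls Spawn Objects at the SpawnSpeed interval.
; Each call spawns one BP_Bounce at a random point inside the Box component's scaled extent around the actor's location, with a random rotation.
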(event EventBeginPlay
  ;[1 1 1] Spawn A B C
  (if (Variables|Default|GetSpawn%20toggle)
    (Utilities|Time|SetTimerbyFunctionName 0 "Spawn Objects" (Variables|Default|GetSpawn%20Speed) true)))

(fn ConstructionScript)

(fn SpawnObjects
  (Game|SpawnActorfromClass "/Game/BallCollect/Blueprints/BounceBall/BP_Bounce.BP_Bounce_C" (Math|Transform|MakeTransform (Math|Random|RandomPointinBoundingBox (Transformation|GetActorLocation) (Components|Box|GetScaledBoxExtent (Variables|Default|GetBox))) (Math|Random|RandomRotator true) "1.000000,1.000000,1.000000") "Undefined" 0 0))