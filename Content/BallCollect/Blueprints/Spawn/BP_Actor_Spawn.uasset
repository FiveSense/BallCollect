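; BP_Actor_Spawn is a spawner actor in BallCollect that repeatedly spawns actors at random points inside its box.
; When SpawnToggle is on, BeginPlay starts a looping timer by function name at SpawnSpeed intervals.
; Each tick of the timer calls Spawn Objects, which spawns every class in GetABCBP within the Box extents around the actor's location.
; The EventGraph also holds an empty SpawnObject event and disconnected leftover spawn, timer and Scale nodes.
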(event Custom|Spawn%20Object
  ;[1 1 1] Error Spawn object
)

(event EventBeginPlay
  ;[1 1 1] Spawn A B C
  (if (Variables|Default|GetSpawn%20toggle)
    (Utilities|Time|SetTimerbyFunctionName 0 "Spawn Objects" (Variables|Default|GetSpawn%20Speed) true)))

(fn ConstructionScript)

(fn SpawnObjects
  (for _array_element (Variables|Default|GetGet%20ABC_BP)
    (Game|SpawnActorfromClass _array_element (Math|Transform|MakeTransform (Math|Random|RandomPointinBoundingBox (Transformation|GetActorLocation) (Components|Box|GetScaledBoxExtent (Variables|Default|GetBox))) "0, 0, 0" "1,1,1") "Undefined" 0 0)))