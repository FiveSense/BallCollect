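; Reads orientation from an Arduino (PILAR) over a serial port and drives the first player's control rotation with it.
; A fast looping timer parses each line as a rotator and median-filters the last seven samples via their forward-vector components.
; A one-time delayed calibration sets the offset, recording roll and yaw on base level 0 or using fixed values otherwise.
; Repeated parse failures reopen the port, and EndPlay closes it.
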(event Custom|CustomEvent_0
  (bind _arduino (Variables|Default|GetArduino))
  ;[1 1 1] PILAR is working!
  (Utilities|IsValid _arduino
    (:Is%20Valid
      (bind (_bsuccess _returnvalue) (Class|Serial|Readln _arduino))
      (if (.OutIsValid (Math|Conversions|ToRotator(Quat) _returnvalue))
        (Variables|Default|SetfalseTimes 0)
        (bind _output_get (Variables|Default|SetArduinoRotate (.OutConvertedRotator (Math|Conversions|ToRotator(Quat) _returnvalue))))
        (bind _output_get_2 (Variables|Default|SetFilterRotation_7 (Variables|Default|GetFilterRotation_6)))
        (bind _output_get_3 (Variables|Default|SetFilterRotation_6 (Variables|Default|GetFilterRotation_5)))
        (bind _output_get_4 (Variables|Default|SetFilterRotation_5 (Variables|Default|GetFilterRotation_4)))
        (bind _output_get_5 (Variables|Default|SetFilterRotation_4 (Variables|Default|GetFilterRotation_3)))
        (bind _output_get_6 (Variables|Default|SetFilterRotation_3 (Variables|Default|GetFilterRotation_2)))
        (bind _output_get_7 (Variables|Default|SetFilterRotation_2 (Variables|Default|GetFilterRotation_1)))
        (bind _output_get_8 (Variables|Default|SetFilterRotation_1 _output_get))
        (bind _res (CallFunction|MedianFilter (Utilities|Array|MakeArray _output_get_2 _output_get_3 _output_get_4 _output_get_5 _output_get_6 _output_get_7 _output_get_8)))
        (bind _output_get_9 (Variables|Default|SetRecentRotater _res))
        (Utilities|FlowControl|Sequence
          (:then_0
            (Utilities|FlowControl|DoOnce false
              (:Completed
                (switch int (Variables|Default|GetBaseLevel)
                  (:Default
                    (Utilities|FlowControl|Delay 1.0)
                    (Variables|Default|SetRecordV "0,-15.000000,155.000000"))
                  (:0
                    (Utilities|FlowControl|Delay 1.0)
                    (bind _output_get_10 (Variables|Default|SetRecord (Variables|Default|GetRecentRotater)))
                    (Variables|Default|SetRecordV (Math|Vector|MakeVector (.Roll (Math|Rotator|BreakRotator (Variables|Default|GetRecentRotater))) 0.0 (.Yaw (Math|Rotator|BreakRotator (Variables|Default|GetRecentRotater)))))
                    (Development|PrintString (Utilities|String|ToString(Rotator) _output_get_10)))))))
          (:then_1
            (Pawn|SetControlRotation (Game|GetPlayerController 0) (Math|Rotator|MakeRotator (.x (+ (- (Math|Vector|MakeVector (.Roll (Math|Rotator|BreakRotator _output_get_9)) (.Pitch (Math|Rotator|BreakRotator _output_get_9)) (.Yaw (Math|Rotator|BreakRotator _output_get_9))) (Variables|Default|GetRecordV)) "0.000000,15.000000,-155.000000")) (* (.y (+ (- (Math|Vector|MakeVector (.Roll (Math|Rotator|BreakRotator _output_get_9)) (.Pitch (Math|Rotator|BreakRotator _output_get_9)) (.Yaw (Math|Rotator|BreakRotator _output_get_9))) (Variables|Default|GetRecordV)) "0.000000,15.000000,-155.000000")) -1.0) (* (.z (+ (- (Math|Vector|MakeVector (.Roll (Math|Rotator|BreakRotator _output_get_9)) (.Pitch (Math|Rotator|BreakRotator _output_get_9)) (.Yaw (Math|Rotator|BreakRotator _output_get_9))) (Variables|Default|GetRecordV)) "0.000000,15.000000,-155.000000")) 1.0)))))
        (else
          (bind _output_get_11 (Variables|Default|SetfalseTimes (+ (Variables|Default|GetfalseTimes) 1)))
          (if (> _output_get_11 200)
            (CallFunction|OpenPort (Variables|Default|Getport))
            (Variables|Default|SetfalseTimes 0)))))))

(event EventTick
  (params (DeltaSeconds :type Float%20%28single-precision%29))
  ;[1 1 1] PILAR is working!
)

(event EventEndPlay
  (params (EndPlayReason :type EEndPlayReason%20Enum :default "Destroyed"))
  (bind _arduino (Variables|Default|GetArduino))
  ;[1 1 1] PILAR is working!
  ;;[1 1 1] If PILAR is enabled, we need to stop it.
  (Utilities|IsValid _arduino
    (:Is%20Valid
      (Class|Serial|Close _arduino))))

(event EventBeginPlay
  (Utilities|FlowControl|Sequence
    (:then_0
      (if (Variables|Default|GetisVaild)
        (CallFunction|OpenPort (Variables|Default|Getport))))
    (:then_1
      ;[1 1 1] PILAR is working!
      (Utilities|Time|SetTimerbyEvent (delegate Custom|CustomEvent_0) 0.01 true))))

(fn ConstructionScript)

(fn MedianFilter
  (params (A :type Array%20of%20Rotators))
  (bind _returnvalue (Utilities|Array|Length A))
  (bind _array (Utilities|Array|MakeArray))
  (bind _returnvalue_2 (/ _returnvalue 2))
  (Variables|Default|SetArrayX _array)
  (Variables|Default|SetArrayY _array)
  (Variables|Default|SetArrayZ _array)
  (for _array_element A
    (Utilities|Array|Add (Variables|Default|GetArrayX) (.X (Math|Vector|BreakVector (Math|Rotator|GetRotationXVector _array_element))))
    (Utilities|Array|Add (Variables|Default|GetArrayY) (.Y (Math|Vector|BreakVector (Math|Rotator|GetRotationXVector _array_element))))
    (Utilities|Array|Add (Variables|Default|GetArrayZ) (.Z (Math|Vector|BreakVector (Math|Rotator|GetRotationXVector _array_element)))))
  (Class|LowEntryExtendedStandardLibrary|SortFloatArrayDirectly (Variables|Default|GetArrayX) false)
  (Class|LowEntryExtendedStandardLibrary|SortFloatArrayDirectly (Variables|Default|GetArrayY) false)
  (Class|LowEntryExtendedStandardLibrary|SortFloatArrayDirectly (Variables|Default|GetArrayZ) false)
  (return (Math|Conversions|RotationFromXVector (Math|Vector|MakeVector (Utilities|Array|Get(acopy) (Variables|Default|GetArrayX) _returnvalue_2) (Utilities|Array|Get(acopy) (Variables|Default|GetArrayY) _returnvalue_2) (Utilities|Array|Get(acopy) (Variables|Default|GetArrayZ) _returnvalue_2)))))

(fn CheckRotate)

(fn OpenPort
  (params (port :type Integer))
  (Utilities|IsValid (Variables|Default|GetArduino)
    (:Is%20Valid
      (Class|Serial|Close (Variables|Default|GetArduino)))
    (:Is%20Not%20Valid
      _))
  (bind (_bopened _returnvalue) (Class|Serial|OpenComPort port 19200))
  (if _bopened
    (bind _output_get (Variables|Default|SetArduino _returnvalue))
    (Class|Serial|Flush _output_get)
    (Development|PrintString "Welcome to use PILAR!!!!!!!!!!!!!!!!!!!!!!!!!!!!!" true true "(R=0.000000,G=0.660000,B=1.000000,A=1.000000)" 2.0)
    (Variables|Default|SetTickCount 0)
    (Development|PrintString (Utilities|String|ToString(Integer) (Class|Serial|GetPort _output_get)))
    (else
      (Development|PrintString "Failed to initialize PILAR" true true "(R=1.000000,G=0.100000,B=0.278808,A=1.000000)" 2e+01))))